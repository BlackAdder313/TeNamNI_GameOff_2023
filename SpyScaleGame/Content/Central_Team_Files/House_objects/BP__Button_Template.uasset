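; Template Blueprint for a level exit button that reflects puzzle completion and loads the next level when pressed.
; Tick polls IsComplete to swap the green or red material and, once complete, notifies BP_PlayerSpy if required triggers exist.
; Pressing disables player movement, plays the HUD level transition and loads LevelName after a delay, pulsing the Puzzle_Advance global parameter.
; The press handler itself does not check completion.
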(event `self.ReceiveTick`
  (params (DeltaSeconds :type "Float (single-precision)"))
  (bind _returnvalue (`self.IsComplete`))
  (`PrimitiveComponent.SetMaterial` (`self.CanExitButton`) 0 (select `bool` _returnvalue :`false` "/Game/Central_Team_Files/House_objects/Materials/Red_Square_Button_64x64_Texture_Mat.Red_Square_Button_64x64_Texture_Mat" :`true` "/Game/Central_Team_Files/House_objects/Materials/Green_Circle_Butrton_64x64_Texture_Mat.Green_Circle_Butrton_64x64_Texture_Mat" :!type "MaterialInterface Object Reference"))
  (if _returnvalue
    ;[1 1 1] If the button has no required triggered,  this should be handled manually per level
    (`/Engine/EditorBlueprintResources/StandardMacros.DoOnce` false
      (:`Completed`
        (if (`KismetMathLibrary.Conv_IntToBool` (`KismetArrayLibrary.Array_Length` (`self.RequiredTriggers`)))
          (bind _asbp_player_spy (cast `/Game/Central_Team_Files/Player/BP_PlayerSpy` (`GameplayStatics.GetPlayerCharacter` 0)))
          (`/Game/Central_Team_Files/Player/BP_PlayerSpy.OnTriggersComplete` _asbp_player_spy))))))

(event `self.BP_OnButtonPressed`
  (bind _returnvalue (`GameplayStatics.GetPlayerCharacter` 0))
  (`|ExecutionSequence`
    (:`then_0`
      (`FMODBlueprintStatics.SetGlobalParameterByName` "Puzzle_Advance" 1.0))
    (:`then_1`
      (`CharacterMovementComponent.DisableMovement` (`Character.CharacterMovement` _returnvalue)))
    (:`then_2`
      (bind _asbp_player_spy (cast `/Game/Central_Team_Files/Player/BP_PlayerSpy` _returnvalue))
      (`/Game/Central_Team_Files/HUD_Menus/PlayerHUD.LevelTransition` (`/Game/Central_Team_Files/Player/BP_PlayerSpy.PlayerHUD` _asbp_player_spy)))
    (:`then_3`
      (`KismetSystemLibrary.Delay` 5.0)
      (`FMODBlueprintStatics.SetGlobalParameterByName` "Puzzle_Advance")
      (`GameplayStatics.OpenLevel` (`self.Level Name`)))))

(fn `UserConstructionScript`)