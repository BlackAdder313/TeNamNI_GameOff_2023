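; BP_Surveillance is a surveillance camera house object that watches the player and drives timed voicelines.
; A physics handle grabs the Camera component at BeginPlay, and Tick turns its target rotation to face the player character.
; BeginPlay also starts a 2D FMOD voiceline event, then two delayed branches briefly pulse the global VoiceNum parameter minutes into play to select lines.
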(event `self.ReceiveBeginPlay`
  (bind _camera (`self.Camera`))
  (`FMODBlueprintStatics.PlayEvent2D` "/Game/FMOD/Events/SFX/Voicelines.Voicelines")
  (`PhysicsHandleComponent.GrabComponentAtLocationWithRotation` (`self.PhysicsHandle`) _camera "None" (`SceneComponent.K2_GetComponentLocation` _camera) (`SceneComponent.K2_GetComponentRotation` _camera))
  (`|ExecutionSequence`
    (:`then_0`
      (`KismetSystemLibrary.Delay` 120.0)
      (`FMODBlueprintStatics.SetGlobalParameterByName` "VoiceNum" 1.0))
    (:`then_1`
      (`KismetSystemLibrary.Delay` 360.0)
      (`FMODBlueprintStatics.SetGlobalParameterByName` "VoiceNum" 2.0)))
  (`KismetSystemLibrary.Delay` 0.2)
  (`FMODBlueprintStatics.SetGlobalParameterByName` "VoiceNum" 0.0))

(event `self.ReceiveTick`
  (params (DeltaSeconds :type "Float (single-precision)"))
  (bind _returnvalue (`GameplayStatics.GetPlayerCharacter` 0))
  (`/Engine/EditorBlueprintResources/StandardMacros.IsValid` _returnvalue
    (:`Is Valid`
      (`PhysicsHandleComponent.SetTargetRotation` (`self.PhysicsHandle`) (`KismetMathLibrary.FindLookAtRotation` (`self.K2_GetActorLocation`) (`self.K2_GetActorLocation` _returnvalue))))))

(fn `UserConstructionScript`)