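; Pressure-button trigger template that sinks as it nears completion and reacts when its completed state changes.
; Box overlap begin and end feed the trigger's TriggerOverlap and EndOverlap functions.
; Tick eases the button mesh's height toward a depth scaled by completion percentage, dropping further once complete.
; Completion changes set the global Button_Press parameter and switch the button's emissive glow on or off.
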(event `self.ReceiveTick`
  (params (DeltaSeconds :type "Float (single-precision)"))
  (bind _buttonmesh (`self.ButtonMesh`))
  (bind (_relativelocation_x _relativelocation_y _relativelocation_z) (`KismetMathLibrary.BreakVector` (`SceneComponent.RelativeLocation` _buttonmesh)))
  (`/Engine/EditorBlueprintResources/StandardMacros.IsValid` _buttonmesh
    (:`Is Valid`
      (`SceneComponent.K2_SetRelativeLocation` _buttonmesh (`KismetMathLibrary.MakeVector` 0.0 0.0 (`KismetMathLibrary.FInterpTo` _relativelocation_z (`KismetMathLibrary.SelectFloat` -30.0 (`KismetMathLibrary.Lerp` 0.0 -17.0 (`self.GetCompletePercentage`)) (`self.IsComplete`)) DeltaSeconds 7.0)) false false))))

(event `self.Sphere.OnComponentBeginOverlap`
  (params (OverlappedComponent :type "PrimitiveComponent Object Reference") (OtherActor :type "Actor Object Reference") (OtherComp :type "PrimitiveComponent Object Reference") (OtherBodyIndex :type Integer) (bFromSweep :type Boolean) (SweepResult :type "HitResult Structure (by ref)")))

(event `self.Sphere.OnComponentEndOverlap`
  (params (OverlappedComponent :type "PrimitiveComponent Object Reference") (OtherActor :type "Actor Object Reference") (OtherComp :type "PrimitiveComponent Object Reference") (OtherBodyIndex :type Integer)))

(event `self.On_CompleteChange`
  (params (bHasCompleted :type Boolean))
  (if bHasCompleted
    (`FMODBlueprintStatics.SetGlobalParameterByName` "Button_Press")
    (`FMODBlueprintStatics.SetGlobalParameterByName` "Button_Press" 1.0)
    (`MeshComponent.SetScalarParameterValueOnMaterials` (`self.ButtonMesh`) "EmmisiveScalar" 0.5)
    (else
      (`FMODBlueprintStatics.SetGlobalParameterByName` "Button_Press" 2.0)
      (`MeshComponent.SetScalarParameterValueOnMaterials` (`self.ButtonMesh`) "EmmisiveScalar" 0.0))))

(event `self.Box.OnComponentBeginOverlap`
  (params (OverlappedComponent :type "PrimitiveComponent Object Reference") (OtherActor :type "Actor Object Reference") (OtherComp :type "PrimitiveComponent Object Reference") (OtherBodyIndex :type Integer) (bFromSweep :type Boolean) (SweepResult :type "HitResult Structure (by ref)"))
  (`self.BP_TriggerOverlap` null OtherActor OtherComp OtherBodyIndex bFromSweep SweepResult))

(event `self.Box.OnComponentEndOverlap`
  (params (OverlappedComponent :type "PrimitiveComponent Object Reference") (OtherActor :type "Actor Object Reference") (OtherComp :type "PrimitiveComponent Object Reference") (OtherBodyIndex :type Integer))
  (`self.BP_EndOverlap` OverlappedComponent OtherActor OtherComp OtherBodyIndex))

(fn `UserConstructionScript`)