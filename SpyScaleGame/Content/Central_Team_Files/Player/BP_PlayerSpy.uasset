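; BP_PlayerSpy is the player spy Blueprint, which adds the HUD on BeginPlay and drives grow and shrink laser gun effects.
; Mouse buttons and gamepad triggers toggle IsShootingAnim, a flag for the animation Blueprint.
; Holding right mouse spawns grow laser Niagara systems at the Muzzle, left mouse shrink ones, repeating each frame through zero-delay loops.
; The gamepad triggers spawn no VFX, and the Gun VFX and SFX graph is empty.
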(event `self.ReceiveBeginPlay`
  (`|ExecutionSequence`
    (:`then_0`
      ;[1 1 1] HUD
      (bind _returnvalue (`|CreateWidget` "/Game/Central_Team_Files/HUD_Menus/PlayerHUD.PlayerHUD_C"))
      (`UserWidget.AddToViewport` _returnvalue 0))))

(event `Key|LeftMouseButton`
  (params (Key :type "Key Structure"))
  ;[1 1 1] Feeds into the BP Anim
  (:`Pressed`
    (set `self.IsShootingAnim` true :!label _label))
  (:`Released`
    (set `self.IsShootingAnim` false :!label _label_2)))

(event `Key|RightMouseButton`
  (params (Key :type "Key Structure"))
  ;[1 1 1] Grow VFX system
  (:`Pressed`
    (set `self.FireButtonPressed` true)
    (if (`self.CanFire`)
      (`self.GrowLaserVFX` :!label _label_3)
      (`KismetSystemLibrary.Delay` 0.0)
      (set `self.CanFire` true)
      (if (`self.FireButtonPressed`)
        (goto _label_3))))
  (:`Released`
    (set `self.FireButtonPressed` false)))

(event `Key|RightMouseButton`
  (params (Key :type "Key Structure"))
  ;[1 1 1] Feeds into the BP Anim
  (:`Pressed`
    (goto _label))
  (:`Released`
    (goto _label_2)))

(event `Key|Gamepad_LeftTrigger`
  (params (Key :type "Key Structure"))
  ;[1 1 1] Feeds into the BP Anim
  (:`Pressed`
    (goto _label))
  (:`Released`
    (goto _label_2)))

(event `Key|Gamepad_RightTrigger`
  (params (Key :type "Key Structure"))
  ;[1 1 1] Feeds into the BP Anim
  (:`Pressed`
    (goto _label))
  (:`Released`
    (goto _label_2)))

(event `Key|LeftMouseButton`
  (params (Key :type "Key Structure"))
  ;[1 1 1] Shrink VFX system
  (:`Pressed`
    (set `self.FireButtonPressedShrink` true)
    (if (`self.CanFireShrink`)
      (`self.ShrinkLaserVFX` :!label _label_4)
      (`KismetSystemLibrary.Delay` 0.0)
      (set `self.CanFireShrink` true)
      (if (`self.FireButtonPressedShrink`)
        (goto _label_4))))
  (:`Released`
    (set `self.FireButtonPressedShrink` false)))

(fn `GrowLaserVFX`
  (bind _muzzle (`self.Muzzle`))
  (`NiagaraFunctionLibrary.SpawnSystemAtLocation` "/Game/Central_Team_Files/Player/Shrink_Grow_Gun/Grow_Laser.Grow_Laser" (`SceneComponent.K2_GetComponentLocation` _muzzle) (`SceneComponent.K2_GetComponentRotation` _muzzle)))

(fn `Gun VFX and SFX`)

(fn `ShrinkLaserVFX`
  (bind _muzzle (`self.Muzzle`))
  (`NiagaraFunctionLibrary.SpawnSystemAtLocation` "/Game/Central_Team_Files/Player/Shrink_Grow_Gun/Shrink_Laser.Shrink_Laser" (`SceneComponent.K2_GetComponentLocation` _muzzle) (`SceneComponent.K2_GetComponentRotation` _muzzle)))

(fn `UserConstructionScript`)